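; Player controller that lets the player switch control between the BP_Project0Pawn actors in the level using number keys 1 to 5.
; On BeginPlay it caches all those pawns in the Players array.
; Each key passes its number as a zero-based array index to PossessPlayer, so the first pawn has no key.
; PossessPlayer always unpossesses first, so an invalid index leaves no pawn possessed.
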(event `self.ReceiveBeginPlay`
  (bind _outactors (`GameplayStatics.GetAllActorsOfClass` "/Game/01BluePrints/BP_Project0Pawn.BP_Project0Pawn_C"))
  (set `self.Players` _outactors))

(event `Key|One`
  (params (Key :type "Key Structure"))
  (:`Pressed`
    (`self.PossessPlayer` 1)))

(event `Key|Two`
  (params (Key :type "Key Structure"))
  (:`Pressed`
    (`self.PossessPlayer` 2)))

(event `Key|Three`
  (params (Key :type "Key Structure"))
  (:`Pressed`
    (`self.PossessPlayer` 3)))

(event `Key|Four`
  (params (Key :type "Key Structure"))
  (:`Pressed`
    (`self.PossessPlayer` 4)))

(event `Key|Five`
  (params (Key :type "Key Structure"))
  (:`Pressed`
    (`self.PossessPlayer` 5)))

(fn `PossessPlayer`
  (params (PlayerIndex :type Integer))
  (`self.UnPossess`)
  (if (`KismetArrayLibrary.Array_IsValidIndex` (`self.Players`) (`local.PlayerIndex`))
    (`self.Possess` (`|GetArrayItem` (`self.Players`) (`local.PlayerIndex`)))))

(fn `UserConstructionScript`)